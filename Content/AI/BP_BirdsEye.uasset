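; BP_BirdsEye is a pawn that a player can take over from their character and move vertically.
; Activate, from the Roaming or Idle state, stores the character and its PlayerController, possesses this pawn and switches State to Possessed.
; It also sets the view target to the PlayerCameraManager itself rather than to the pawn.
; The MoveUp axis feeds up-vector input into FloatingPawnMovement.
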(event Input|AxisEvents|InputAxisMoveUp
  (params (AxisValue :type Float%20%28single-precision%29))
  (Class|PawnMovementComponent|AddInputVector (Variables|Default|GetFloatingPawnMovement) (* (Math|Vector|VectorUp) AxisValue) false))

(fn ConstructionScript)

(fn Activate
  (params (Character :type Character%20Object%20Reference))
  (switch Utilities|FlowControl|Switch|SwitchonStates (Variables|Default|GetState)
    (:NewEnumerator0
      _)
    (:NewEnumerator2
      _))
  (bind _output_get (Variables|Default|SetPlayer Character))
  (bind _asplayer_controller (Utilities|Casting|CastToPlayerController (Pawn|GetController _output_get)))
  (bind _output_get_2 (LocalVariables|SetPlayer%20Controller _asplayer_controller))
  (Pawn|Possess _output_get_2 self)
  (Game|Player|SetViewTargetwithBlend _output_get_2 (Variables|/Script/Engine.PlayerController|GetPlayerCameraManager (LocalVariables|GetPlayer%20Controller)) 0.0 "VTBlend_Linear" 0.0 false)
  (Variables|Default|SetState "NewEnumerator1"))